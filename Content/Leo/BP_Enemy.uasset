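; Enemy for the Froggy game mode that patrols a spline path and penalizes the player's timer on contact.
; Tick advances a distance along PathBP's spline, wrapping or reversing at the ends after configurable delays; the construction script also snaps it onto the path.
; Player overlap passes a DoOnce, then a Loop macro calls the game mode's Second every 0.1 seconds until the AddedSeconds count is reached, then re-arms.
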(event OnComponentBeginOverlap(Sphere1)
  (params (OverlappedComponent :type Primitive%20Component%20Object%20Reference) (OtherActor :type Actor%20Object%20Reference) (OtherComp :type Primitive%20Component%20Object%20Reference) (OtherBodyIndex :type Integer) (bFromSweep :type Boolean) (SweepResult :type Hit%20Result%20Structure%20%28by%20ref%29))
  ;[1 1 1] Kill
  (Utilities|Casting|CastToBP_Player_Froggy OtherActor)
  ;;[1 1 1] Timer
  (Utilities|FlowControl|DoOnce false :!label _label
    (:Completed
      (Utilities|Loop :!label _label_2
        (:true
          (goto _label Reset))
        (:false
          (Default|Second (Variables|Default|GetGamemode))
          (Utilities|FlowControl|Delay 0.1)
          (goto _label_2))))))

(event Custom|UpdatePosition
  (bind _pathbp (Variables|Default|GetPathBP))
  ;[1 1 1] UpdatePosition
  (Utilities|IsValid _pathbp
    (:Is%20Valid
      (Transformation|SetActorLocation (Spline|GetLocationatDistanceAlongSpline (Variables|/Game/Leo/BP_PathSpline.BP_PathSpline_C|GetSpline _pathbp) (Variables|Default|GetDistanceAlongSpline) "World") false false))))

(event Custom|Move
  ;[1 1 1] Movement
  (CallFunction|UpdatePosition)
  (if (Variables|Default|GetIsMovingForward)
    (if (< (Variables|Default|GetDistanceAlongSpline) (Spline|GetSplineLength (Variables|/Game/Leo/BP_PathSpline.BP_PathSpline_C|GetSpline (Variables|Default|GetPathBP))))
      (Variables|Default|SetDistanceAlongSpline (+ (Variables|Default|GetDistanceAlongSpline) (* (Utilities|Time|GetWorldDeltaSeconds) (Variables|Default|GetSpeed))))
      (elif (Variables|Default|GetDoesLoop)
        (Utilities|FlowControl|Delay (Variables|Default|GetWaitAtEndpoint))
        (Variables|Default|SetDistanceAlongSpline 0.0)
        (else
          (Utilities|FlowControl|Delay (Variables|Default|GetWaitAtEndpoint))
          (Variables|Default|SetIsMovingForward false))))
    (elif (> (Variables|Default|GetDistanceAlongSpline) 0.0)
      (Variables|Default|SetDistanceAlongSpline (- (Variables|Default|GetDistanceAlongSpline) (* (Utilities|Time|GetWorldDeltaSeconds) (Variables|Default|GetSpeed))))
      (elif (Variables|Default|GetDoesLoop)
        (Utilities|FlowControl|Delay (Variables|Default|GetWaitAtStartpoint))
        (Variables|Default|SetDistanceAlongSpline (Spline|GetSplineLength (Variables|/Game/Leo/BP_PathSpline.BP_PathSpline_C|GetSpline (Variables|Default|GetPathBP))))
        (else
          (Utilities|FlowControl|Delay (Variables|Default|GetWaitAtStartpoint))
          (Variables|Default|SetIsMovingForward true))))))

(event EventBeginPlay
  (bind _asbp_gm_froggy (Utilities|Casting|CastToBP_GM_Froggy (Game|GetGameMode)))
  (Variables|Default|SetGamemode _asbp_gm_froggy))

(event EventTick
  (params (DeltaSeconds :type Float%20%28single-precision%29))
  ;[1 1 1] Tick
  (if (Variables|Default|GetCanMove)
    (CallFunction|Move)))

(fn ConstructionScript
  (CallFunction|UpdatePosition))