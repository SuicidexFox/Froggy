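; BP_Lilypad is a level lilypad that shrinks away when the Froggy player overlaps it and grows back afterwards.
; A DoOnce gates the overlap, adding a short delay if the player's JumpTrigger is set, before a timeline lerps scale from its BeginPlay value to zero.
; When any actor's overlap ends, a delay runs, then the DoOnce resets and the timeline reverses.
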(event Collision|EventActorBeginOverlap
  (params (OtherActor :type Actor%20Object%20Reference))
  (bind _asbp_player_froggy (Utilities|Casting|CastToBP_Player_Froggy OtherActor))
  (Utilities|FlowControl|DoOnce false
    (:Completed
      (if (Variables|/Game/Mary/Player/BP_Player_Froggy.BP_Player_Froggy_C|GetJumpTrigger _asbp_player_froggy)
        (Utilities|FlowControl|Delay 1.0)
        (bind _value (Timeline|Scale Play)
          (:Update
            (Transformation|SetActorScale3D (Math|Vector|Lerp(Vector) (Variables|Default|GetStartTransform) "0, 0, 0" _value))))
        (else
          (Timeline|Scale Play))))))

(event Collision|EventActorEndOverlap
  (params (OtherActor :type Actor%20Object%20Reference))
  (Utilities|FlowControl|Delay 3.0)
  (Utilities|FlowControl|Sequence
    (:then_0
      (Utilities|FlowControl|DoOnce false) ; enters at Reset
    )
    (:then_1
      (bind _value (Timeline|Scale Reverse)
        (:Update
          (Transformation|SetActorScale3D (Math|Vector|Lerp(Vector) (Variables|Default|GetStartTransform) "0, 0, 0" _value)))))))

(event EventBeginPlay
  (Variables|Default|SetStartTransform (Transformation|GetActorScale3D)))

(fn ConstructionScript)