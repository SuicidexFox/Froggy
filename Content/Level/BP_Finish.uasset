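; BP_Finish is a level goal trigger that moves the Froggy player through difficulty tiers.
; BeginPlay caches the current level name.
; On overlap with BP_Player_Froggy it plays the finish Niagara effect, waits briefly, then matches that hardcoded name to open a random level from the next tier (Easy, Normal, Hard, Epic).
; Finishing an Epic level instead pushes WBP_Leaderboard onto the HUD overlay's widget stack.
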(event EventBeginPlay
  (bind _returnvalue (Game|GetCurrentLevelName true))
  (bind _output_get (Variables|Default|SetCurrentLevel _returnvalue))
  (Development|PrintString _output_get))

(event Collision|EventActorBeginOverlap
  (params (OtherActor :type Actor%20Object%20Reference))
  (bind _currentlevel (Variables|Default|GetCurrentLevel))
  (bind _currentlevel_2 (Variables|Default|GetCurrentLevel))
  (bind _currentlevel_3 (Variables|Default|GetCurrentLevel))
  (bind _currentlevel_4 (Variables|Default|GetCurrentLevel))
  (bind _asbp_player_froggy (Utilities|Casting|CastToBP_Player_Froggy OtherActor))
  (Default|FinishNiagara _asbp_player_froggy)
  (Utilities|FlowControl|Delay 2.0)
  (if (or (Utilities|Enum|Equal(Enum) "Lvl_Easy_1" _currentlevel_4) (Utilities|Enum|Equal(Enum) _currentlevel_4 "Lvl_Easy_2"))
    (Game|OpenLevel(byObjectReference) (.OutItem (Utilities|Array|Random (Variables|Default|GetNormalLevel))))
    (elif (or (Utilities|Enum|Equal(Enum) "Lvl_Normal_1" _currentlevel) (Utilities|Enum|Equal(Enum) _currentlevel "Lvl_Normal_2"))
      (Game|OpenLevel(byObjectReference) (.OutItem (Utilities|Array|Random (Variables|Default|GetHardLevel))))
      (elif (or (Utilities|Enum|Equal(Enum) "Lvl_Hard_1" _currentlevel_2) (Utilities|Enum|Equal(Enum) _currentlevel_2 "Lvl_Hard_2"))
        (Game|OpenLevel(byObjectReference) (.OutItem (Utilities|Array|Random (Variables|Default|GetEpicLevel))))
        (elif (or (Utilities|Enum|Equal(Enum) "Lvl_Epic_1" _currentlevel_3) (Utilities|Enum|Equal(Enum) _currentlevel_3 "Lvl_Epic_2"))
          (bind _asbp_hud_froggy (Utilities|Casting|CastToBP_HUD_Froggy (HUD|GetHUD (Game|GetPlayerController 0))))
          (Class|CommonActivatableWidgetContainerBase|AddWidget (Variables|/Game/HUD/HUD_Overlay.HUD_Overlay_C|GetWidget_Stack (Variables|/Game/Mary/BP_HUD_Froggy.BP_HUD_Froggy_C|GetHUDOverlay _asbp_hud_froggy)) "/Game/HUD/WBP_Leaderboard.WBP_Leaderboard_C"))))))

(fn ConstructionScript)