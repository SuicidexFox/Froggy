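; BP_CollectableSpeed is a pickup that grants the speed ability to BP_Player_Froggy when that player overlaps it.
; The overlap plays a Collect timeline that pulls the pickup toward the player's current location while shrinking it to zero scale.
; When the timeline finishes, it sets CanSpeed on the player and destroys itself.
; A DoOnce on the overlap's second sequence branch drives nothing, and PlayEvent2D is empty.
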(event Collision|EventActorBeginOverlap
  (params (OtherActor :type Actor%20Object%20Reference))
  (Utilities|FlowControl|Sequence
    (:then_0
      (bind _asbp_player_froggy (Utilities|Casting|CastToBP_Player_Froggy OtherActor))
      (bind _value (Timeline|Collect Play)
        (:Update
          (Transformation|SetActorLocation (Math|Vector|Lerp(Vector) (Transformation|GetActorLocation) (Transformation|GetActorLocation _asbp_player_froggy) _value) false false)
          (Transformation|SetActorScale3D (Math|Vector|Lerp(Vector) "1.000000,1.000000,1.000000" "0, 0, 0" _value)))
        (:Finished
          (Variables|/Game/Mary/Player/BP_Player_Froggy.BP_Player_Froggy_C|SetCanSpeed _asbp_player_froggy true)
          (Actor|DestroyActor))))
    (:then_1
      (Utilities|FlowControl|DoOnce false))))

(fn ConstructionScript)