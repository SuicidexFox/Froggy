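; BP_GI_Froggy is a game instance that manages persistent settings for Master, Music and SFX bus volumes.
; Init loads or creates a BP_SG_Settings save object, polls each tick until the game mode is valid, then applies the volumes.
; Shutdown saves to the "Settings" slot, but Init's existence check uses the misspelled "Settiungs", so loading depends on that other slot existing.
; CallToGameInstance returns the instance itself.
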(event Custom|SetupVolume
  (bind _sg_settings (Variables|Default|GetSG%20Settings))
  (Class|FMODBlueprintStatics|BusSetVolume "/Game/FMOD/Buses/Master.Master" (Variables|/Game/Mary/BP_SG_Settings.BP_SG_Settings_C|GetMasterVolume _sg_settings))
  (Class|FMODBlueprintStatics|BusSetVolume "/Game/FMOD/Buses/Master/Music.Music" (Variables|/Game/Mary/BP_SG_Settings.BP_SG_Settings_C|GetMusicVolume _sg_settings))
  (Class|FMODBlueprintStatics|BusSetVolume "/Game/FMOD/Buses/Master/SFX.SFX" (Variables|/Game/Mary/BP_SG_Settings.BP_SG_Settings_C|GetSFXVolume _sg_settings)))

(event EventShutdown
  (SaveGame|SaveGametoSlot (Variables|Default|GetSG%20Settings) "Settings"))

(event EventInit
  (bind _returnvalue (SaveGame|DoesSaveGameExist "Settiungs"))
  (if _returnvalue
    (bind _returnvalue_2 (SaveGame|LoadGamefromSlot "Settings"))
    (bind _asbp_sg_settings (Utilities|Casting|CastToBP_SG_Settings _returnvalue_2))
    (Variables|Default|SetSG%20Settings _asbp_sg_settings)
    (else
      (bind _returnvalue_3 (SaveGame|CreateSaveGameObject "/Game/Mary/BP_SG_Settings.BP_SG_Settings_C"))
      (Variables|Default|SetSG%20Settings _returnvalue_3)))
  (Utilities|IsValid (Game|GetGameMode) :!label _label
    (:Is%20Valid
      (CallFunction|SetupVolume))
    (:Is%20Not%20Valid
      (Utilities|FlowControl|DelayUntilNextTick)
      (goto _label))))

(fn CalltoGameInstance
  (return self))