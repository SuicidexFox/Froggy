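; BP_PC_Froggy is the player controller for Froggy that sets up input and opens the pause menu.
; On BeginPlay it adds the ActionMap_Froggy mapping context to the Enhanced Input local player subsystem.
; When IA_Pause starts, it pushes WBP_Main onto the Froggy HUD overlay's widget stack, then pushes WBP_Pause onto that widget's menu stack.
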(event Input|EnhancedActionEvents|EnhancedInputActionIA_Pause
  (params (ActionValue :type Boolean) (ElapsedSeconds :type Float%20%28double-precision%29) (TriggeredSeconds :type Float%20%28double-precision%29) (InputAction :type Input%20Action%20Object%20Reference :default "/Game/Mary/Input/IA_Pause.IA_Pause"))
  (:Started
    (bind _asbp_hud_froggy (Utilities|Casting|CastToBP_HUD_Froggy (HUD|GetHUD (Game|GetPlayerController 0))))
    (bind _returnvalue (Class|CommonActivatableWidgetContainerBase|AddWidget (Variables|/Game/HUD/HUD_Overlay.HUD_Overlay_C|GetWidget_Stack (Variables|/Game/Mary/BP_HUD_Froggy.BP_HUD_Froggy_C|GetHUDOverlay _asbp_hud_froggy)) "/Game/HUD/WBP_Main.WBP_Main_C"))
    (Class|CommonActivatableWidgetContainerBase|AddWidget (Variables|/Game/HUD/WBP_Main.WBP_Main_C|GetMenu_Stack _returnvalue) "/Game/HUD/WBP_Pause.WBP_Pause_C")))

(event EventBeginPlay
  (bind _returnvalue (PlayerController|LocalPlayerSubsystems|GetEnhancedInputLocalPlayerSubsystem))
  (Utilities|IsValid _returnvalue
    (:Is%20Valid
      (Input|AddMappingContext _returnvalue "/Game/Mary/Input/ActionMap_Froggy.ActionMap_Froggy" 0 "(bIgnoreAllPressedKeysUntilRelease=True,bForceImmediately=False,bNotifyUserSettings=False)"))))

(fn ConstructionScript)