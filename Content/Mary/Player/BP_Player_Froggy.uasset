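; BP_Player_Froggy is the player frog, with Enhanced Input movement (optionally inverted), a quack sound, and timed transform and sprint abilities.
; Transform temporarily enables jumping, otherwise a no-jump montage plays, while sprint briefly raises walk speed; both use DoOnce plus Delay cooldowns.
; Forward movement follows control yaw but strafing uses a fixed world axis.
; Both transform mesh swaps set FrogHuman, and the AnimClass swaps are disconnected.
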(event Input|EnhancedActionEvents|EnhancedInputActionIA_Transform
  (params (ActionValue :type Boolean) (ElapsedSeconds :type Float%20%28double-precision%29) (TriggeredSeconds :type Float%20%28double-precision%29) (InputAction :type Input%20Action%20Object%20Reference :default "/Game/Mary/Input/IA_Transform.IA_Transform"))
  (bind _mesh (Variables|Character|GetMesh))
  (:Started
    (if (and (Variables|Inputs|GetCanMove) (Variables|Inputs|GetCanTransfrom))
      (Utilities|FlowControl|DoOnce false :!label _label
        (:Completed
          (Variables|Inputs|SetJumpTrigger true)
          (Components|SkeletalMesh|SetSkeletalMeshAsset _mesh "/Game/Mary/Player/Frog/FrogHuman.FrogHuman")
          (Utilities|FlowControl|Delay 5.0) ; TransformTime
          (Components|SkeletalMesh|SetSkeletalMeshAsset _mesh "/Game/Mary/Player/HumanFrog/FrogHuman.FrogHuman")
          (Variables|Inputs|SetJumpTrigger false)
          (Utilities|FlowControl|Delay 5.0) ; Cooldown
          (goto _label Reset)))
      (else
        (Development|PrintString "Bool noch nicht bereit")))))

(event Input|EnhancedActionEvents|EnhancedInputActionIA_Voice
  (params (ActionValue :type Boolean) (ElapsedSeconds :type Float%20%28double-precision%29) (TriggeredSeconds :type Float%20%28double-precision%29) (InputAction :type Input%20Action%20Object%20Reference :default "/Game/Mary/Input/IA_Voice.IA_Voice"))
  (:Started
    (if (Variables|Inputs|GetCanMove)
      (Class|FMODBlueprintStatics|PlayEvent2D "/Game/FMOD/Events/Char/Quak.Quak"))))

(event Input|EnhancedActionEvents|EnhancedInputActionIA_Jump
  (params (ActionValue :type Boolean) (ElapsedSeconds :type Float%20%28double-precision%29) (TriggeredSeconds :type Float%20%28double-precision%29) (InputAction :type Input%20Action%20Object%20Reference :default "/Game/Mary/Input/IA_Jump.IA_Jump"))
  (:Started
    (if (Math|Boolean|ANDBoolean (Variables|Inputs|GetCanMove) (Variables|Inputs|GetJumpTrigger) (AI|Components|NavMovement|IsMovingonGround (Variables|Character|GetCharacterMovement)))
      (Character|Jump)
      (else
        (Animation|PlayAnimMontage "/Game/Mary/Player/HumanFrog/Animation/AM_NoJump.AM_NoJump" 1.0 "None")))))

(event Input|EnhancedActionEvents|EnhancedInputActionIA_Move
  (params (ActionValue :type Vector%202D%20Structure) (ElapsedSeconds :type Float%20%28double-precision%29) (TriggeredSeconds :type Float%20%28double-precision%29) (InputAction :type Input%20Action%20Object%20Reference :default "/Game/Mary/Input/IA_Move.IA_Move"))
  (bind _invert (Variables|Inputs|GetInvert))
  (bind _returnvalue (Math|Float|SelectFloat -1.0 1.0 _invert))
  (if (Variables|Inputs|GetCanMove)
    (Pawn|Input|AddMovementInput (Math|Vector|GetForwardVector (Math|Rotator|MakeRotator 0.0 0.0 (.yaw (Pawn|GetControlRotation :!class /Script/Engine.Pawn)))) (* (.x ActionValue) _returnvalue) false) ; W/S
    (Pawn|Input|AddMovementInput "0.000000,90.000000,0.000000" (* (.y ActionValue) _returnvalue) false) ; A/D
  ))

(event Input|EnhancedActionEvents|EnhancedInputActionIA_Sprint
  (params (ActionValue :type Boolean) (ElapsedSeconds :type Float%20%28double-precision%29) (TriggeredSeconds :type Float%20%28double-precision%29) (InputAction :type Input%20Action%20Object%20Reference :default "/Game/Mary/Input/IA_Sprint.IA_Sprint"))
  (bind _charactermovement (Variables|Character|GetCharacterMovement))
  (:Started
    (if (and (Variables|Inputs|GetCanMove) (Variables|Inputs|GetCanSpeed))
      (Utilities|FlowControl|DoOnce false :!label _label
        (:Completed
          (Variables|/Script/Engine.CharacterMovementComponent|SetMaxWalkSpeed _charactermovement 8e+02)
          (Utilities|FlowControl|Delay 5.0)
          (Variables|/Script/Engine.CharacterMovementComponent|SetMaxWalkSpeed _charactermovement 5e+02)
          (Utilities|FlowControl|Delay 5.0) ; Cooldown
          (goto _label Reset))))))

(event EventBeginPlay
  (Variables|Default|SetStartTransform (Transformation|GetActorTransform)))

(fn ConstructionScript)