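; Collectable pickup that flies into BP_Player_Froggy on overlap and appears to unlock jumping.
; The Collect timeline pulls it from its current location toward the player's live position while shrinking it to zero scale.
; When the timeline finishes, it overwrites the player's CharacterMovement nav agent properties, with jump as the only enabled movement capability, then destroys itself.
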(event Collision|EventActorBeginOverlap
  (params (OtherActor :type Actor%20Object%20Reference))
  (bind _asbp_player_froggy (Utilities|Casting|CastToBP_Player_Froggy OtherActor))
  (bind _value (Timeline|Collect Play)
    (:Update
      (Transformation|SetActorLocation (Math|Vector|Lerp(Vector) (Transformation|GetActorLocation) (Transformation|GetActorLocation _asbp_player_froggy) _value) false false)
      (Transformation|SetActorScale3D (Math|Vector|Lerp(Vector) "1.000000,1.000000,1.000000" "0, 0, 0" _value)))
    (:Finished
      (Variables|/Script/Engine.NavMovementComponent|SetNavAgentProps (Variables|/Script/Engine.Character|GetCharacterMovement _asbp_player_froggy) (Utilities|Struct|MakeNavAgentProperties -1.0 -1.0 -1.0 0.5 "None" false true false false false))
      (Actor|DestroyActor))))

(fn ConstructionScript)